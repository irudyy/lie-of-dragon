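; BP_Lava is a lava hazard that hurts the player on contact.
; When a BP_ValeriiHUD_Player_Angle overlaps its Box, it casts player pawn 0 to that class and calls LavaDamage, leaving the damage logic to the player.
; A PickedUp handler refreshes NewHUD's score text and destroys the actor, but its OnPickedUp call is unwired, and the Damage function is empty.
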(event OnComponentBeginOverlap(Box)
  (params (OverlappedComponent :type Primitive%20Component%20Object%20Reference) (OtherActor :type Actor%20Object%20Reference) (OtherComp :type Primitive%20Component%20Object%20Reference) (OtherBodyIndex :type Integer) (bFromSweep :type Boolean) (SweepResult :type Hit%20Result%20Structure%20%28by%20ref%29))
  ;[0.15 0.15 0.15 0.5] Lava  settings
  (if (Class|GameplayStatics|ObjectIsA OtherActor "/Game/LevelPrototyping/HUD/BP_ValeriiHUD_Player_Angle.BP_ValeriiHUD_Player_Angle_C")
    (bind _asbp_valerii_hud_player_angle (Utilities|Casting|CastToBP_ValeriiHUD_Player_Angle (Game|Player|GetPlayerPawn 0)))
    (Default|LavaDamage _asbp_valerii_hud_player_angle)))

(event EventBeginPlay)

(event Collision|EventActorBeginOverlap
  (params (OtherActor :type Actor%20Object%20Reference)))

(event EventTick
  (params (DeltaSeconds :type Float%20%28single-precision%29)))

(fn ConstructionScript)

(fn Damage)