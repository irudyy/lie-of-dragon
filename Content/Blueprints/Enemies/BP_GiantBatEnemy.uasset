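; Giant bat enemy that tracks its health and marks a zone tied to the player's quick-time event.
; Overlapping QTEZone registers the bat with BP_ValeriiHUD_Player_Angle through EnterBatZone, and leaving calls ExitBatZone.
; ApplyQTEDamage subtracts a fixed per-success amount from health, clamped between zero and max, and prints a debug HP readout.
; The bat contains no death handling.
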(event OnComponentBeginOverlap(QTEZone)
  (params (OverlappedComponent :type Primitive%20Component%20Object%20Reference) (OtherActor :type Actor%20Object%20Reference) (OtherComp :type Primitive%20Component%20Object%20Reference) (OtherBodyIndex :type Integer) (bFromSweep :type Boolean) (SweepResult :type Hit%20Result%20Structure%20%28by%20ref%29))
  (bind _asbp_valerii_hud_player_angle (Utilities|Casting|CastToBP_ValeriiHUD_Player_Angle OtherActor)
    (:then
      (Default|EnterBatZone _asbp_valerii_hud_player_angle self))
    (:CastFailed
      (Development|PrintString "Ошибка каста" true true "(R=1.000000,G=0.003496,B=0.047784,A=1.000000)"))))

(event OnComponentEndOverlap(QTEZone)
  (params (OverlappedComponent :type Primitive%20Component%20Object%20Reference) (OtherActor :type Actor%20Object%20Reference) (OtherComp :type Primitive%20Component%20Object%20Reference) (OtherBodyIndex :type Integer))
  (bind _asbp_valerii_hud_player_angle (Utilities|Casting|CastToBP_ValeriiHUD_Player_Angle OtherActor))
  (Default|ExitBatZone _asbp_valerii_hud_player_angle self))

(event Custom|ApplyQTEDamage
  (Variables|Default|SetCurrentHealth (Math|Float|Clamp(Float) (- (Variables|Default|GetCurrentHealth) (Variables|Default|GetDamagePerSuccess)) 0.0 (Variables|Default|GetMaxHealth)))
  (Development|PrintString (Utilities|String|ToString(Text) (Utilities|Text|FormatText "Bat HP: {HP}" (Math|Float|Clamp(Float) (- (Variables|Default|GetCurrentHealth) (Variables|Default|GetDamagePerSuccess)) 0.0 (Variables|Default|GetMaxHealth))))))

(event EventBeginPlay
  (Variables|Default|SetCurrentHealth (Variables|Default|GetMaxHealth)))

(fn ConstructionScript)